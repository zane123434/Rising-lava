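; BP_MySplinePlatform is a platform actor that moves along a spline once play begins.
; BeginPlay calls PlatformStart, which plays a timeline whose SplineDistence track is scaled by spline length to set the mesh's world location without sweeping.
; The construction script applies the StaticMesh and Material variables to the platform mesh, so each placed instance can have its own look.
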(event Custom|Platform%20Start
  (bind _spline (Variables|Default|GetSpline))
  (bind _spline_distence (Timeline|Motion%20Timeline Play)
    (:Update
      (Transformation|SetWorldLocation (Variables|Default|GetPlatform%20Mesh) (Spline|GetLocationatDistanceAlongSpline _spline (* _spline_distence (Spline|GetSplineLength _spline)) "World") false false))))

(event EventBeginPlay
  (CallFunction|PlatformStart))

(event Collision|EventActorBeginOverlap
  (params (OtherActor :type Actor%20Object%20Reference)))

(event EventTick
  (params (DeltaSeconds :type Float%20%28single-precision%29)))

(fn ConstructionScript
  (bind _platform_mesh (Variables|Default|GetPlatform%20Mesh))
  (Components|StaticMesh|SetStaticMesh _platform_mesh (Variables|Default|GetStatic%20Mesh))
  (Rendering|Material|SetMaterial _platform_mesh 0 (Variables|Default|GetMaterial)))