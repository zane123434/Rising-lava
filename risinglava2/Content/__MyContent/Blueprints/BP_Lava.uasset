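; BP_Lava is a rising lava hazard that sends the player back to a checkpoint on contact.
; Box overlap by a ThirdPersonCharacter teleports it above its CurrentCheckpoint and prints a death message.
; On BeginPlay, MoveComponentTo moves the mesh over MoveSpeed, using Destanation's world location as the relative target.
; The logic to alternate between Location1 and Location2 is disconnected, so the move does not loop.
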(event OnComponentBeginOverlap(Box)
  (params (OverlappedComponent :type Primitive%20Component%20Object%20Reference) (OtherActor :type Actor%20Object%20Reference) (OtherComp :type Primitive%20Component%20Object%20Reference) (OtherBodyIndex :type Integer) (bFromSweep :type Boolean) (SweepResult :type Hit%20Result%20Structure%20%28by%20ref%29))
  ;[1 1 1] Respawn
  (bind _asthird_person_character (Utilities|Casting|CastToThirdPersonCharacter OtherActor))
  (Transformation|SetActorLocation _asthird_person_character (+ (Transformation|GetActorLocation (Variables|/Game/ThirdPersonBP/Blueprints/ThirdPersonCharacter.ThirdPersonCharacter_C|GetCurrent%20Checkpoint _asthird_person_character)) "0, 0,200.000000") false false)
  (Development|PrintString "You Died"))

(event EventBeginPlay
  ;[1 1 1] Rising Lava
  (Components|MoveComponentTo (Variables|Debug|GetStaticMeshComponent) (Transformation|GetActorLocation (Variables|Default|GetDestanation)) "0, 0, 0" false false (Variables|Default|GetMove%20Speed) false)
  (if (== (Variables|Default|GetDestanation) (Variables|Default|GetLocation1))
    _))

(fn ConstructionScript)